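; BP_ItemBase is the base item actor in LittleCooks, providing state-change functions for other code to call; its event graph is empty.
; MarkRetired flags it consumed with a cash-register sound, while MarkAbsorbed flags it consumed, hides it and disables collision.
; PromoteToHeld enables physics and full collision via GetBody's root-component cast; DemoteToLoose disables physics on RootBody, leaving query-only collision.
; Both physics transitions zero linear and angular velocity.
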(event EventBeginPlay)

(event Collision|EventActorBeginOverlap
  (params (OtherActor :type Actor%20Object%20Reference)))

(event EventTick
  (params (DeltaSeconds :type Float%20%28single-precision%29)))

(fn ConstructionScript)

(fn MarkRetired
  (Variables|Default|SetbConsumed true)
  (Audio|PlaySound2D "/Game/LittleCooks/Sounds/Cash_Register_1-2_Cue.Cash_Register_1-2_Cue" 1.0 1.0 0.0 0 0))

(fn MarkAbsorbed
  (Variables|Default|SetbConsumed true)
  (Collision|SetActorEnableCollision false)
  (Rendering|SetActorHiddenInGame true))

(fn DemotetoLoose
  (bind _rootbody (Variables|Default|GetRootBody))
  (Physics|SetPhysicsLinearVelocity _rootbody "0, 0, 0" false "None")
  (Class|PrimitiveComponent|SetPhysicsAngularVelocityinDegrees _rootbody "0, 0, 0" false "None")
  (Physics|SetSimulatePhysics _rootbody false)
  (Collision|SetCollisionEnabled _rootbody "QueryOnly"))

(fn PromotetoHeld
  (bind _body (CallFunction|GetBody))
  (Collision|SetCollisionEnabled _body "QueryAndPhysics")
  (Physics|SetSimulatePhysics _body true)
  (Physics|SetPhysicsLinearVelocity _body "0, 0, 0" false "None")
  (Class|PrimitiveComponent|SetPhysicsAngularVelocityinDegrees _body "0, 0, 0" false "None"))

(fn GetBody
  (bind _as프리미티브_컴포넌트 (Utilities|Casting|CastToPrimitiveComponent (Variables|Transformation|GetRootComponent)))
  (return _as프리미티브_컴포넌트))
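; Rice item actor for a cooking game that represents a clump of grains and can merge with other rice on contact.
; Setting the grain count rebuilds an instanced mesh and scales the capsule by the count's cube root, drawing a debug capsule.
; Overlapping another rice item forwards both item indices to the GameState registry for merging.
; While held, it is teleported to a given transform with physics off and query-only collision.
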(event OnComponentBeginOverlap(RootBody)
  (params (OverlappedComponent :type Primitive%20Component%20Object%20Reference) (OtherActor :type Actor%20Object%20Reference) (OtherComp :type Primitive%20Component%20Object%20Reference) (OtherBodyIndex :type Integer) (bFromSweep :type Boolean) (SweepResult :type Hit%20Result%20Structure%20%28by%20ref%29))
  (bind _asbp_item_rice (Utilities|Casting|CastToBP_Item_Rice OtherActor))
  (bind _asbp_game_state_cooking (Utilities|Casting|CastToBP_GameState_Cooking (Game|GetGameState)))
  (Default|GetRegistry _asbp_game_state_cooking)
  (Default|TryMergeonContact (Variables|/Game/LittleCooks/Framework/BP_GameState_Cooking.BP_GameState_Cooking_C|GetRegistry _asbp_game_state_cooking) (Variables|Default|GetItemIndex) (Variables|BP_Item_Rice_C|GetItemIndex _asbp_item_rice)))

(event EventBeginPlay
  (bind _rootbody (Variables|Default|GetRootBody))
  (Variables|Default|SetBaseCapsuleRadius (Class|CapsuleComponent|GetUnscaledCapsuleRadius _rootbody))
  (Variables|Default|SetBaseCapsuleHalfHeight (Components|Capsule|GetUnscaledCapsuleHalfHeight _rootbody))
  (Physics|SetSimulatePhysics _rootbody false)
  (Collision|SetCollisionEnabled _rootbody "QueryOnly")
  (CallFunction|RebuildGrainVisual))

(event Collision|EventActorBeginOverlap
  (params (OtherActor :type Actor%20Object%20Reference)))

(event EventTick
  (params (DeltaSeconds :type Float%20%28single-precision%29)))

(fn ConstructionScript)

(fn FollowHeldTransform
  (params (Location :type Vector) (Rotation :type Rotator))
  (Physics|SetSimulatePhysics (Variables|Default|GetRootBody) false)
  (Collision|SetCollisionEnabled (Variables|Default|GetRootBody) "QueryOnly")
  (Transformation|SetActorLocationAndRotation Location Rotation false true))

(fn RebuildGrainVisual
  (bind _graincount (Variables|Default|GetGrainCount))
  (bind _basecapsuleradius (Variables|Default|GetBaseCapsuleRadius))
  (bind _basecapsulehalfheight (Variables|Default|GetBaseCapsuleHalfHeight))
  (bind _graincount_2 (Variables|Default|GetGrainCount))
  (bind _returnvalue (Math|Conversions|ToFloat(Integer) _graincount_2))
  (bind _returnvalue_2 (Math|Float|Power _returnvalue 0.3333))
  (bind _returnvalue_3 (* _basecapsuleradius _returnvalue_2))
  (bind _returnvalue_4 (Math|Float|Max(Float) _returnvalue_3 _basecapsulehalfheight))
  (Components|InstancedStaticMesh|ClearInstances (Variables|Default|GetGrainISM))
  (for _index (range 0 (- _graincount 1))
    (Components|InstancedStaticMesh|AddInstance (Variables|Default|GetGrainISM) (Class|RiceMath|GrainTransformfor _index _graincount (Variables|Default|GetBaseExtent) (Variables|Default|GetGrainScale)) false)
    (Components|Capsule|SetCapsuleSize (Variables|Default|GetRootBody) _returnvalue_3 _returnvalue_4 true)
    (Rendering|Debug|DrawDebugCapsule (Transformation|GetActorLocation) _returnvalue_4 _returnvalue_3 "0, 0, 0" "(R=1.000000,G=1.000000,B=1.000000,A=1.000000)" 2.0 0.0)))

(fn SetGrainCount
  (params (N :type Integer))
  (Variables|Default|SetGrainCount N)
  (CallFunction|RebuildGrainVisual))
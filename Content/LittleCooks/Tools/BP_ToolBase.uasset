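; Base hand tool for the cooking game: attaches to the overlapping character and handles networked rice holding, with chopsticks granting a pinch ability.
; The grabber moves rice by PhysicsHandle and streams its transform on a timer, while other machines interpolate it.
; The server resolves grains via RiceController, force-releases previous holders and attempts station delivery.
; Dropped rice is watched until rest or timeout, then its final transform is multicast.
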(event OnComponentBeginOverlap(InteractionBox)
  (params (OverlappedComponent :type Primitive%20Component%20Object%20Reference) (OtherActor :type Actor%20Object%20Reference) (OtherComp :type Primitive%20Component%20Object%20Reference) (OtherBodyIndex :type Integer) (bFromSweep :type Boolean) (SweepResult :type Hit%20Result%20Structure%20%28by%20ref%29))
  (Utilities|Casting|CastToPawn OtherActor)
  (Networking|SwitchHasAuthority
    (:Authority
      (Actor|SetOwner OtherActor)
      (if (not (Utilities|IsValid (Variables|Default|GetOwnerCharacter)))
        (CallFunction|GetOwnerCharacter)
        (CallFunction|OnEquip)))))

(event Custom|Client_ForceRelease
  (if (Variables|Default|GetbIAmGrabbing)
    (Development|PrintString (Utilities|String|Append "FORCE RELEASE, " (Utilities|GetDisplayName self)) true true "(R=0.000000,G=0.660000,B=1.000000,A=1.000000)" 5.0)
    (Physics|Components|PhysicsHandle|ReleaseComponent (Variables|Default|GetPhysicsHandle))
    (Variables|Default|SetbIAmGrabbing false)
    (Variables|Default|SetHeldRice 0)
    (Utilities|Time|ClearandInvalidateTimerbyHandle (Variables|Default|GetPushTimerHandle))))

(event Custom|Server_StartPinch
  (params (Index :type Integer))
  (Audio|PlaySound2D "/Game/LittleCooks/Sounds/Whoosh_1-1.Whoosh_1-1" 1.0 1.0 0.0 0 0)
  (bind _asbp_game_state_cooking (Utilities|Casting|CastToBP_GameState_Cooking (Game|GetGameState)))
  (Default|GetRiceController _asbp_game_state_cooking)
  (bind _tool (Default|FindHolderOf (Variables|/Game/LittleCooks/Framework/BP_GameState_Cooking.BP_GameState_Cooking_C|GetRiceController _asbp_game_state_cooking) Index))
  (Utilities|IsValid _tool
    (:Is%20Valid
      (if (!= _tool self)
        (CallFunction|ClientForceRelease _tool)
        (Variables|BP_ToolBase_C|SetHeldRiceIndex _tool -1)
        (bind _rice (Default|GetRicebyIndex (Variables|/Game/LittleCooks/Framework/BP_GameState_Cooking.BP_GameState_Cooking_C|GetRiceController _asbp_game_state_cooking) Index :!label _label))
        (Utilities|IsValid _rice
          (:Is%20Valid
            (Variables|Default|SetbIsUsingTool true)
            (Variables|Default|SetHeldRiceIndex Index)
            (CallFunction|ApplyHeldRiceIndex)))))
    (:Is%20Not%20Valid
      (goto _label))))

(event Custom|Server_FinishRelease
  (params (ReleasedIndex :type Integer) (RestTransform :type Transform))
  (Variables|Default|SetWatchedRice 0)
  (Variables|Default|SetWatchedIndex -1)
  (Variables|Default|SetHeldRiceIndex -1)
  (CallFunction|ApplyHeldRiceIndex)
  (bind _asbp_game_state_cooking (Utilities|Casting|CastToBP_GameState_Cooking (Game|GetGameState)))
  (Default|GetRiceController _asbp_game_state_cooking)
  (Default|MulticastSetRiceRest (Variables|/Game/LittleCooks/Framework/BP_GameState_Cooking.BP_GameState_Cooking_C|GetRiceController _asbp_game_state_cooking) ReleasedIndex (.location RestTransform) (.rotation RestTransform)))

(event Custom|BeginDropWatch
  (Physics|Components|PhysicsHandle|ReleaseComponent (Variables|Default|GetPhysicsHandle))
  (if (Utilities|IsValid (Variables|Default|GetHeldRice))
    (Variables|Default|SetRestTicks 0)
    (Variables|Default|SetWatchTicks 0)
    (Variables|Default|SetWatchedRice (Variables|Default|GetHeldRice))
    (Variables|Default|SetWatchedIndex (Variables|Default|GetHeldRiceIndex))
    (bind _returnvalue (Utilities|Time|SetTimerbyEvent (delegate Custom|WatchForRest) 0.1 true))
    (bind _output_get (Variables|Default|SetRestTimerHandle _returnvalue))
    (else
      (CallFunction|FinishDrop))))

(event Custom|BeginTracking
  (bind _returnvalue (Utilities|Time|SetTimerbyEvent (delegate Custom|PushHeldTransform) 0.05 true))
  (Variables|Default|SetPushTimerHandle _returnvalue))

(event Custom|Server_UpdateHeld
  (params (Loc :type Vector) (Rot :type Rotator))
  (Variables|Default|SetHeldRiceLocation Loc)
  (Variables|Default|SetHeldRiceRotation Rot))

(event Custom|PushHeldTransform
  (bind _heldrice (Variables|Default|GetHeldRice))
  (bind _ricecapsule (Variables|/Game/LittleCooks/Items/BP_Item_Rice.BP_Item_Rice_C|GetRiceCapsule _heldrice))
  (Physics|Components|PhysicsHandle|SetTargetLocation (Variables|Default|GetPhysicsHandle) (CallFunction|GetToolGrabTarget))
  (CallFunction|ServerUpdateHeld (Transformation|GetWorldLocation _ricecapsule) (Transformation|GetWorldRotation _ricecapsule)))

(event Custom|Server_StopPinch
  (bind _heldriceindex (Variables|Default|GetHeldRiceIndex))
  (Variables|Default|SetbIsUsingTool false)
  (if (>= _heldriceindex 0)
    (bind _asbp_game_state_cooking (Utilities|Casting|CastToBP_GameState_Cooking (Game|GetGameState)))
    (Default|GetRiceController _asbp_game_state_cooking)
    (bind _rice (Default|GetRicebyIndex (Variables|/Game/LittleCooks/Framework/BP_GameState_Cooking.BP_GameState_Cooking_C|GetRiceController _asbp_game_state_cooking) _heldriceindex))
    (Utilities|IsValid _rice
      (:Is%20Valid
        (if (> (Utilities|Array|Length (Collision|GetOverlappingActors _rice "/Game/LittleCooks/Stations/BP_DeliveryStation.BP_DeliveryStation_C" :!class /Script/Engine.Actor)) 0)
          (Default|TryDeliver (Utilities|Array|Get(acopy) (Collision|GetOverlappingActors _rice "/Game/LittleCooks/Stations/BP_DeliveryStation.BP_DeliveryStation_C" :!class /Script/Engine.Actor)) _rice))))))

(event Custom|WatchForRest
  (Utilities|IsValid (Variables|Default|GetWatchedRice)
    (:Is%20Valid
      (Variables|Default|SetWatchTicks (+ (Variables|Default|GetWatchTicks) 1))
      (bind _returnvalue (Physics|GetPhysicsLinearVelocity (Variables|/Game/LittleCooks/Items/BP_Item_Rice.BP_Item_Rice_C|GetRiceCapsule (Variables|Default|GetWatchedRice)) "None"))
      (if (< (Math|Vector|VectorLength _returnvalue) 0.0)
        (Variables|Default|SetRestTicks (+ (Variables|Default|GetRestTicks) 1))
        (else
          (Variables|Default|SetRestTicks 0)))
      (if (or (>= (Variables|Default|GetRestTicks) 3) (> (Variables|Default|GetWatchTicks) 100))
        (CallFunction|FinishDrop)))
    (:Is%20Not%20Valid
      (Utilities|Time|ClearandInvalidateTimerbyHandle (stale Custom|BeginDropWatch _output_get)))))

(event Custom|FinishDrop
  (bind _watchedrice (Variables|Default|GetWatchedRice))
  (Utilities|Time|ClearandInvalidateTimerbyHandle (Variables|Default|GetRestTimerHandle))
  (Utilities|Time|ClearandInvalidateTimerbyHandle (Variables|Default|GetPushTimerHandle))
  (if (Utilities|IsValid _watchedrice)
    (CallFunction|ServerFinishRelease (Variables|/Game/LittleCooks/Items/BP_Item_Rice.BP_Item_Rice_C|GetRiceIndex _watchedrice) (Transformation|GetActorTransform _watchedrice))
    (Utilities|IsValid (Variables|Default|GetHeldRice)
      (:Is%20Valid
        (Default|DemotetoLoose (Variables|Default|GetHeldRice)))))
  (Variables|Default|SetbIAmGrabbing false)
  (Variables|Default|SetHeldRice 0))

(event EventBeginPlay
  (Development|PrintString (Utilities|String|Append "controller valid: " (Utilities|String|ToString(Boolean) (Utilities|IsValid 0))) false false "(R=0.000000,G=0.660000,B=1.000000,A=1.000000)" 1e+01))

(event EventTick
  (params (DeltaSeconds :type Float%20%28single-precision%29))
  (bind _returnvalue (Utilities|Time|GetWorldDeltaSeconds))
  (bind _heldrice (Variables|Default|GetHeldRice))
  (Development|PrintString (Utilities|String|Append "idx = " (Utilities|String|ToString(Integer) (Variables|Default|GetHeldRiceIndex)) " loc = " (Utilities|String|ToString(Vector) (Variables|Default|GetHeldRiceLocation)) " remote = " (Utilities|String|ToString(Boolean) (Utilities|IsValid (Variables|Default|GetHeldRice))) " grab = " (Utilities|String|ToString(Boolean) (Variables|Default|GetbIAmGrabbing)) " auth = " (Utilities|String|ToString(Boolean) (Ability|HasAuthority))) false false "(R=0.000000,G=0.660000,B=1.000000,A=1.000000)" 0.0)
  (if (not (Variables|Default|GetbIAmGrabbing))
    (if (Utilities|IsValid (Variables|Default|GetHeldRice))
      (Transformation|SetActorLocation _heldrice (Math|Interpolation|VInterpTo (Transformation|GetActorLocation _heldrice) (Variables|Default|GetHeldRiceLocation) _returnvalue 2e+01) false true)
      (Transformation|SetWorldRotation (Variables|/Script/Engine.Actor|GetRootComponent _heldrice) (Math|Interpolation|RInterpTo (Transformation|GetActorRotation _heldrice) (Variables|Default|GetHeldRiceRotation) _returnvalue 2e+01) false false))))

(fn ConstructionScript)

(fn OnEquip
  (bind _ownercharacter (Variables|Default|GetOwnerCharacter))
  (bind _output_get (Variables|Default|SetDefaultSceneRoot (Variables|Transformation|GetRootComponent self)))
  (Transformation|AttachComponentToComponent _output_get (Variables|/Script/Engine.Character|GetMesh _ownercharacter) (Utilities|String|StringToName "Hand_R_Socket") "SnapToTarget" "SnapToTarget" "KeepWorld" true)
  (Collision|SetCollisionEnabled (Variables|Default|GetInteractionBox) "NoCollision")
  (Collision|SetCollisionEnabled (Variables|Default|GetMainMesh) "NoCollision")
  (bind _output_get_2 (Variables|/Game/LittleCooks/Player/BP_ThirdPersonCharacter.BP_ThirdPersonCharacter_C|SetEquippedTool _ownercharacter self))
  (Utilities|Casting|CastToBP_Chopsticks _output_get_2)
  (GameplayAbilities|GiveAbility (Variables|/Game/LittleCooks/Player/BP_ThirdPersonCharacter.BP_ThirdPersonCharacter_C|GetAbilitySystem _ownercharacter) "/Game/LittleCooks/Abilities/GA_Chopsticks_Pinch.GA_Chopsticks_Pinch_C" 0 1))

(fn OnUnequip
  (Transformation|DetachFromComponent (Variables|Default|GetDefaultSceneRoot) "KeepRelative" "KeepRelative" "KeepRelative" true))

(fn GetOwnerCharacter
  (if (not (Utilities|IsValid (Variables|Default|GetOwnerCharacter)))
    (bind _asbp_third_person_character (Utilities|Casting|CastToBP_ThirdPersonCharacter (Components|GetOwner)))
    (Variables|Default|SetOwnerCharacter _asbp_third_person_character)))

(fn UseToolStart)

(fn UseToolStop)

(fn OnRepBIsUsingTool
  (if (not (Variables|Default|GetbIAmGrabbing))
    (CallFunction|OnToolUseChanged (Variables|Default|GetbIsUsingTool))))

(fn OnToolUseChanged
  (params (bUsing :type Boolean)))

(fn GetToolGrabTarget
  (return "0, 0, 0"))

(fn ApplyHeldRiceIndex
  (if (not (Variables|Default|GetbIAmGrabbing))
    (if (== (Variables|Default|GetHeldRiceIndex) -1)
      (if (Utilities|IsValid (Variables|Default|GetHeldRice))
        (Default|DemotetoLoose (Variables|Default|GetHeldRice))
        (Variables|Default|SetHeldRice 0))
      (else
        (bind _asbp_game_state_cooking (Utilities|Casting|CastToBP_GameState_Cooking (Game|GetGameState)))
        (Default|GetRiceController _asbp_game_state_cooking)
        (bind _rice (Default|GetRicebyIndex (Variables|/Game/LittleCooks/Framework/BP_GameState_Cooking.BP_GameState_Cooking_C|GetRiceController _asbp_game_state_cooking) (Variables|Default|GetHeldRiceIndex)))
        (if (Utilities|IsValid _rice)
          (Variables|Default|SetHeldRice _rice)
          (Physics|SetSimulatePhysics (Variables|/Game/LittleCooks/Items/BP_Item_Rice.BP_Item_Rice_C|GetRiceCapsule _rice) false))))))

(fn OnRepHeldRiceIndex
  (CallFunction|ApplyHeldRiceIndex))
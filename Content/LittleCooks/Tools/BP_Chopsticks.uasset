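; BP_Chopsticks is a hand tool that pinches and carries BP_ItemBase items.
; Using it plays a timeline that rotates both sticks closed, grabs the first item overlapping the tip box unless consumed, and reports it to the server by index.
; A PhysicsHandle follows the tip each tick while an item is held.
; Releasing reverses the timeline, notifies the server and starts a drop watch; tool-use changes also drive the pinch visual.
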(event Custom|StartPinch
  (bind _tipgrabbox (Variables|Default|GetTipGrabBox))
  (bind _tipgrabbox_2 (Variables|Default|GetTipGrabBox))
  (bind _overlappingactors (Collision|GetOverlappingActors _tipgrabbox_2 "/Game/LittleCooks/Items/BP_ItemBase.BP_ItemBase_C" :!class /Script/Engine.PrimitiveComponent))
  (Utilities|Time|ClearandInvalidateTimerbyHandle (Variables|Default|GetRestTimerHandle))
  (Development|PrintString (Utilities|String|ToString(Integer) (Utilities|Array|Length _overlappingactors)) false false)
  (CallFunction|SetPinchVisual true)
  (if (> (Utilities|Array|Length (Collision|GetOverlappingActors _tipgrabbox "/Game/LittleCooks/Items/BP_ItemBase.BP_ItemBase_C" :!class /Script/Engine.PrimitiveComponent)) 0)
    (bind _asbp_item_base (Utilities|Casting|CastToBP_ItemBase (Utilities|Array|Get(acopy) _overlappingactors)))
    (if (not (Variables|/Game/LittleCooks/Items/BP_Item_Rice.BP_Item_Rice_C|GetbConsumed _asbp_item_base))
      (Variables|Default|SetbIAmGrabbing true)
      (Default|PromotetoHeld _asbp_item_base)
      (Class|PhysicsHandleComponent|GrabComponentatLocation (Variables|Default|GetPhysicsHandle) (Variables|/Game/LittleCooks/Items/BP_ItemBase.BP_ItemBase_C|GetRootBody _asbp_item_base) "None" (Transformation|GetWorldLocation _tipgrabbox))
      (bind _output_get (Variables|Default|SetHeldItem _asbp_item_base))
      (CallFunction|ServerStartPinch (Variables|/Game/LittleCooks/Items/BP_Item_Rice.BP_Item_Rice_C|GetItemIndex _output_get))
      (CallFunction|BeginTracking)
      (Development|PrintString (Utilities|String|Append "PUSH  held유효= " (Utilities|String|ToString(Boolean) (Utilities|IsValid (Variables|Default|GetHeldItem))) " loc= " (Utilities|String|ToString(Vector) (Transformation|GetWorldLocation (Variables|/Game/LittleCooks/Items/BP_ItemBase.BP_ItemBase_C|GetRootBody (Variables|Default|GetHeldItem))))) false false "(R=0.000000,G=0.660000,B=1.000000,A=1.000000)" 1e+01))
    (else
      (CallFunction|ServerStartPinch -1))))

(event Custom|StopPinch
  (CallFunction|SetPinchVisual false)
  (CallFunction|ServerStopPinch)
  (CallFunction|BeginDropWatch))

(event Custom|SetPinchVisual
  (params (bClosed :type Boolean))
  (if bClosed
    (bind _alpha (Timeline|TM_Pinch Play)
      (:Update
        (Transformation|SetRelativeRotation (Variables|Default|GetStick_Left) (Math|Rotator|CombineRotators (Variables|Default|GetInitailRotLeft) (Math|Rotator|Lerp(Rotator) "0, 0, 0" "-15.000000,0.000000,0.000000" _alpha)) false false)
        (Transformation|SetRelativeRotation (Variables|Default|GetStick_Right) (Math|Rotator|CombineRotators (Variables|Default|GetInitailRotRight) (Math|Rotator|Lerp(Rotator) "0, 0, 0" "15.000000,0.000000,0.000000" _alpha)) false false)))
    (else
      (Timeline|TM_Pinch Reverse))))

(event EventBeginPlay
  (Development|PrintString "chopsticks beginplay" false false "(R=0.000000,G=0.660000,B=1.000000,A=1.000000)" 1e+01)
  (|CallParentFunction)
  (Variables|Default|SetInitailRotLeft (Variables|/Script/Engine.SceneComponent|GetRelativeRotation (Variables|Default|GetStick_Left)))
  (Variables|Default|SetInitailRotRight (Variables|/Script/Engine.SceneComponent|GetRelativeRotation (Variables|Default|GetStick_Right))))

(event Collision|EventActorBeginOverlap
  (params (OtherActor :type Actor%20Object%20Reference))
  (|CallParentFunction OtherActor))

(event EventTick
  (params (DeltaSeconds :type Float%20%28single-precision%29))
  (|CallParentFunction DeltaSeconds)
  (if (Utilities|IsValid (Variables|Default|GetHeldItem))
    (Physics|Components|PhysicsHandle|SetTargetLocation (Variables|Default|GetPhysicsHandle) (Transformation|GetWorldLocation (Variables|Default|GetTipGrabBox)))))

(fn ConstructionScript
  (|CallParentFunction))

(fn UseToolStop
  (|CallParentFunction)
  (CallFunction|StopPinch))

(fn UseToolStart
  (|CallParentFunction)
  (CallFunction|StartPinch))

(fn OnToolUseChanged
  (params (bUsing :type Boolean))
  (CallFunction|SetPinchVisual bUsing))

(fn GetToolGrabTarget
  (return (Transformation|GetWorldLocation (Variables|Default|GetTipGrabBox))))
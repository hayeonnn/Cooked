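; Rice item registry that spawns grains locally on each machine and keeps them in sync by array index.
; The server picks a replicated SpawnSeed, so seeded streams place identical trace-grounded batches in a box, with a checksum printed to verify.
; Index-based multicasts handle merge, delivery, rest transforms and extra rain batches, avoiding per-grain references.
; Merges are server-validated, requiring a tool holding the grain; ApplyDeltas exists but OnRep_RiceDeltas is empty.
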(event Custom|Multicast_SetRiceRest
  (params (Index :type Integer) (Location :type Vector) (Rotation :type Rotator))
  (bind _rice (CallFunction|GetItembyIndex Index))
  (Utilities|IsValid _rice
    (:Is%20Valid
      (Transformation|SetActorLocationAndRotation _rice Location Rotation false true)
      (Physics|SetSimulatePhysics (Variables|/Game/LittleCooks/Items/BP_ItemBase.BP_ItemBase_C|GetRootBody _rice) false)
      (Development|PrintString (Utilities|String|Append "auth = " (Utilities|String|ToString(Boolean) (Ability|HasAuthority)) " index = " (Utilities|String|ToString(Integer) Index) " sent = " (Utilities|String|ToString(Vector) Location) " actual = " (Utilities|String|ToString(Vector) (Transformation|GetActorLocation _rice))) false false "(R=0.000000,G=0.660000,B=1.000000,A=1.000000)" 1e+01)
      (if (Variables|/Game/LittleCooks/Items/BP_Item_Rice.BP_Item_Rice_C|GetbConsumed _rice)
        (Collision|SetActorEnableCollision false)))))

(event Custom|Multicast_MergeRice
  (params (TargetIndex%20 :type Integer) (ConsumedIndex%20 :type Integer) (NewGrainCount%20 :type Integer))
  (bind _rice (CallFunction|GetItembyIndex ConsumedIndex%20))
  (Utilities|IsValid _rice
    (:Is%20Valid
      (Audio|PlaySoundatLocation "/Game/LittleCooks/Sounds/Special_Collectible_26-1_Cue.Special_Collectible_26-1_Cue" (Transformation|GetActorLocation _rice) "0, 0, 0" 1.0 1.0 0.0 0 0 0 0)
      (Default|MarkAbsorbed _rice)
      (bind _rice_2 (CallFunction|GetItembyIndex TargetIndex%20))
      (bind _asbp_item_rice (Utilities|Casting|CastToBP_Item_Rice _rice_2))
      (Default|SetGrainCount _asbp_item_rice NewGrainCount%20))))

(event Custom|Multicast_DeliverRice
  (params (Index%20 :type Integer))
  (bind _rice (CallFunction|GetItembyIndex Index%20))
  (Utilities|IsValid _rice
    (:Is%20Valid
      (Default|MarkRetired _rice))))

(event Custom|Multicast_RainRice
  (params (BatchIndex :type Integer) (Count :type Integer))
  (bind _allitems (Variables|Default|GetAllItems))
  (bind _returnvalue (Utilities|Array|Length _allitems))
  (bind _returnvalue_2 (Utilities|String|ToString(Integer) _returnvalue))
  (Audio|PlaySound2D "/Game/LittleCooks/Sounds/Special_Collectible_9-1_Cue.Special_Collectible_9-1_Cue" 1.0 1.0 0.0 0 0)
  (Development|PrintString (Utilities|String|Append "rain batch : " (Utilities|String|ToString(Integer) BatchIndex) "  count : " (Utilities|String|ToString(Integer) Count) "  before : " _returnvalue_2) false false "(R=0.000000,G=0.660000,B=1.000000,A=1.000000)" 5.0)
  (CallFunction|SpawnRiceBatch (+ BatchIndex 1000 (Variables|Default|GetSpawnSeed)) Count)
  (Development|PrintString (Utilities|String|Append "rain done" "" "  after : " _returnvalue_2) false false "(R=0.000000,G=0.660000,B=1.000000,A=1.000000)" 5.0))

(event EventBeginPlay
  (Networking|SwitchHasAuthority
    (:Authority
      (Variables|Default|SetSpawnSeed (Math|Random|RandomIntegerinRange 0 2000000000))
      (CallFunction|BuildRice))))

(event Collision|EventActorBeginOverlap
  (params (OtherActor :type Actor%20Object%20Reference)))

(event EventTick
  (params (DeltaSeconds :type Float%20%28single-precision%29)))

(fn ConstructionScript)

(fn OnRepSpawnSeed
  (CallFunction|BuildRice))

(fn BuildRice
  (Development|PrintString "start buildRice" false false)
  (if (not (Variables|Default|GetbBuilt))
    (Variables|Default|SetbBuilt true)
    (CallFunction|SpawnRiceBatch (Variables|Default|GetSpawnSeed) (Variables|Default|GetFirstCount))))

(fn PrintChecksum
  (bind _positions (LocalVariables|GetPositions))
  (for _array_element (Variables|Default|GetAllItems)
    (Utilities|IsValid _array_element
      (:Is%20Valid
        (Utilities|Array|Add _positions (Transformation|GetActorLocation _array_element)))))
  (Development|PrintString (Class|RiceMath|RiceChecksumLabel _positions (Variables|Default|GetSpawnSeed) 1.0) true true "(R=0.000000,G=0.660000,B=1.000000,A=1.000000)" 1e+01))

(fn ApplyDeltas
  (for (_array_element _array_index) (Variables|Default|GetRiceDeltas)
    (if (and (>= _array_index 0) (< _array_index (Utilities|Array|Length (Variables|Default|GetAllItems))))
      (bind _asbp_item_rice (Utilities|Casting|CastToBP_Item_Rice (Utilities|Array|Get(acopy) (Variables|Default|GetAllItems) (.index _array_element))))
      (LocalVariables|SetLocalRice _asbp_item_rice)
      (switch Utilities|FlowControl|Switch|SwitchonE_RiceState (.state _array_element)
        (:NewEnumerator0
          (Physics|SetSimulatePhysics (Variables|/Game/LittleCooks/Items/BP_ItemBase.BP_ItemBase_C|GetRootBody (LocalVariables|GetLocalRice)) false)
          (Transformation|SetActorTransform (LocalVariables|GetLocalRice) (.resttransform _array_element) false true))
        (:NewEnumerator1
          (Rendering|SetActorHiddenInGame (LocalVariables|GetLocalRice) true)
          (Collision|SetCollisionEnabled (Variables|/Game/LittleCooks/Items/BP_ItemBase.BP_ItemBase_C|GetRootBody (LocalVariables|GetLocalRice)) "NoCollision"))
        (:NewEnumerator2
          (Collision|SetCollisionEnabled (Variables|/Game/LittleCooks/Items/BP_ItemBase.BP_ItemBase_C|GetRootBody (LocalVariables|GetLocalRice)) "NoCollision"))))))

(fn OnRepRiceDeltas)

(fn GetItembyIndex
  (params (Index :type Integer))
  (bind _self self)
  (if (Utilities|IsValid _self)
    (if (and (>= Index 0) (< Index (Utilities|Array|Length (Variables|BP_ItemRegistry_C|GetAllItems _self))))
      (bind _asbp_item_rice (Utilities|Casting|CastToBP_Item_Rice (Utilities|Array|Get(acopy) (Variables|BP_ItemRegistry_C|GetAllItems _self) Index)))
      (return _asbp_item_rice)
      (else
        (return 0)))))

(fn TryMergeonContact
  (params (HeldIndex :type Integer) (TouchedIndex :type Integer))
  (if (Ability|HasAuthority)
    (Development|PrintString (Utilities|String|Append "MERGE held=" (Utilities|String|ToString(Integer) HeldIndex) " touched=" (Utilities|String|ToString(Integer) TouchedIndex)))
    (if (!= HeldIndex TouchedIndex)
      (bind _rice (CallFunction|GetItembyIndex HeldIndex))
      (bind _asbp_item_rice (Utilities|Casting|CastToBP_Item_Rice _rice))
      (bind _rice_2 (CallFunction|GetItembyIndex TouchedIndex))
      (bind _asbp_item_rice_2 (Utilities|Casting|CastToBP_Item_Rice _rice_2))
      (if (and (not (Variables|/Game/LittleCooks/Items/BP_Item_Rice.BP_Item_Rice_C|GetbConsumed _asbp_item_rice)) (not (Variables|/Game/LittleCooks/Items/BP_Item_Rice.BP_Item_Rice_C|GetbConsumed _asbp_item_rice_2)))
        (CallFunction|GetTools)
        (bind _tool (CallFunction|FindHolderOf HeldIndex))
        (Development|PrintString (Utilities|String|Append "HOLDER= " (Utilities|GetDisplayName _tool)))
        (Utilities|IsValid _tool
          (:Is%20Valid
            (CallFunction|MulticastMergeRice HeldIndex TouchedIndex (+ (Variables|/Game/LittleCooks/Items/BP_Item_Rice.BP_Item_Rice_C|GetGrainCount _asbp_item_rice) (Variables|/Game/LittleCooks/Items/BP_Item_Rice.BP_Item_Rice_C|GetGrainCount _asbp_item_rice_2)))))))))

(fn GetTools
  (if (> (Utilities|Array|Length (Variables|Default|GetTools)) 0)
    (return (Variables|Default|GetTools))
    (else
      (bind _outactors (Actor|GetAllActorsOfClass "/Game/LittleCooks/Tools/BP_ToolBase.BP_ToolBase_C"))
      (for _array_element _outactors
        (Utilities|Array|Add (Variables|Default|GetTools) _array_element))
      (return (Variables|Default|GetTools)))))

(fn SpawnRiceBatch
  (params (Seed :type Integer) (Count :type Integer))
  (bind _spawncenterbox (Variables|Default|GetSpawnCenterBox))
  (bind _allitems (Variables|Default|GetAllItems))
  (Development|PrintString (Utilities|String|Append "seed : " (Utilities|String|ToString(Integer) Seed)) false false "(R=0.000000,G=0.660000,B=1.000000,A=1.000000)" 1e+02)
  (bind _output_get (LocalVariables|SetStream (Math|Random|MakeRandomStream Seed)))
  (Math|Random|SetRandomStreamSeed _output_get Seed)
  (for _index (range 0 (- Count 1))
    (bind (_outhit _returnvalue) (Collision|LineTraceByChannel (+ (Class|KismetMathLibrary|RandomPointinBoundingBoxfromStream _output_get (Transformation|GetWorldLocation _spawncenterbox) (Components|Box|GetScaledBoxExtent _spawncenterbox)) "0.000000,0.000000,200.000000") (- (Class|KismetMathLibrary|RandomPointinBoundingBoxfromStream _output_get (Transformation|GetWorldLocation _spawncenterbox) (Components|Box|GetScaledBoxExtent _spawncenterbox)) "0.000000,0.000000,500.000000") "TraceTypeQuery1" false 0 "None"))
    (if _returnvalue
      (bind _returnvalue_2 (Game|SpawnActorfromClass "/Game/LittleCooks/Items/BP_Item_Rice.BP_Item_Rice_C" (Math|Transform|MakeTransform (.Location (Collision|BreakHitResult _outhit)) (Class|KismetMathLibrary|RandomRotatorfromStream _output_get false) "1.000000,1.000000,1.000000") "AlwaysSpawn" "MultiplyWithRoot" 0 0))
      (Variables|/Game/LittleCooks/Items/BP_Item_Rice.BP_Item_Rice_C|SetItemIndex _returnvalue_2 (Utilities|Array|Length _allitems))
      (Utilities|Array|Add _allitems _returnvalue_2)))
  (Development|PrintString (Utilities|String|Append "rice count: " (Utilities|String|ToString(Integer) (Utilities|Array|Length (Variables|Default|GetAllItems)))) false false "(R=0.000000,G=0.660000,B=1.000000,A=1.000000)" 1e+02)
  (CallFunction|PrintChecksum))

(fn FindHolderOf
  (params (Index :type Integer))
  (if (>= Index 0)
    (bind _tools (CallFunction|GetTools))
    (bind _array_element (Utilities|Array|ForEachLoopwithBreak _tools)
      (:LoopBody
        (if (== (Variables|/Game/LittleCooks/Tools/BP_ToolBase.BP_ToolBase_C|GetHeldItemIndex _array_element) Index)
          (return _array_element))))))
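; BP_DeliveryStation is the station in Little Cooks where rice portions are delivered for score.
; TryDeliver rejects consumed rice and deliveries after the round ends, then has BP_GameState_Cooking grade the shari by grain count.
; It adds to the game state's delivery count and total score, then multicasts the delivered item index through the game state's Registry.
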(event EventBeginPlay)

(event EventTick
  (params (DeltaSeconds :type Float%20%28single-precision%29)))

(fn ConstructionScript)

(fn TryDeliver
  (params (Rice :type BP%20Item%20Rice%20Object%20Reference))
  (if (not (Variables|/Game/LittleCooks/Items/BP_Item_Rice.BP_Item_Rice_C|GetbConsumed Rice))
    (bind _asbp_game_state_cooking (Utilities|Casting|CastToBP_GameState_Cooking (Game|GetGameState)))
    (if (not (Variables|/Game/LittleCooks/Framework/BP_GameState_Cooking.BP_GameState_Cooking_C|GetbRoundOver _asbp_game_state_cooking))
      (bind _score (Default|GradeShari _asbp_game_state_cooking (Variables|/Game/LittleCooks/Items/BP_Item_Rice.BP_Item_Rice_C|GetGrainCount Rice)))
      (Variables|/Game/LittleCooks/Framework/BP_GameState_Cooking.BP_GameState_Cooking_C|SetDelivered _asbp_game_state_cooking (+ (Variables|/Game/LittleCooks/Framework/BP_GameState_Cooking.BP_GameState_Cooking_C|GetDelivered _asbp_game_state_cooking) 1))
      (Variables|/Game/LittleCooks/Framework/BP_GameState_Cooking.BP_GameState_Cooking_C|SetTotalScore _asbp_game_state_cooking (+ (Variables|/Game/LittleCooks/Framework/BP_GameState_Cooking.BP_GameState_Cooking_C|GetTotalScore _asbp_game_state_cooking) _score))
      (Default|GetRegistry _asbp_game_state_cooking)
      (Default|MulticastDeliverRice (Variables|/Game/LittleCooks/Framework/BP_GameState_Cooking.BP_GameState_Cooking_C|GetRegistry _asbp_game_state_cooking) (Variables|/Game/LittleCooks/Items/BP_Item_Rice.BP_Item_Rice_C|GetItemIndex_0 Rice)))))
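; BP_GameState_Cooking is the game state for the LittleCooks cooking game, providing item registry lookup and shari (sushi rice) grading.
; GetRegistry finds the first BP_ItemRegistry actor in the level and caches it when the stored reference is invalid.
; GradeShari passes a grain count and the state's target, per-grain score and penalty settings to a same-named helper, returning score and quality.
; BeginPlay, Tick and the Delivered RepNotify are empty.
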(event EventBeginPlay)

(event EventTick
  (params (DeltaSeconds :type Float%20%28single-precision%29)))

(fn ConstructionScript)

(fn OnRepDelivered)

(fn GetRegistry
  (Development|PrintString (Utilities|String|Append "controller valid: " (Utilities|String|ToString(Boolean) (Utilities|IsValid (Variables|Default|GetRegistry)))) false false "(R=0.000000,G=0.660000,B=1.000000,A=1.000000)" 0.0)
  (if (not (Utilities|IsValid (Variables|Default|GetRegistry)))
    (bind _outactors (Actor|GetAllActorsOfClass "/Game/LittleCooks/Systems/BP_ItemRegistry.BP_ItemRegistry_C"))
    (if (> (Utilities|Array|Length _outactors) 0)
      (Variables|Default|SetRegistry (Utilities|Array|Get(acopy) _outactors)))))

(fn GradeShari
  (params (GrainCount :type Integer))
  (bind _targetgraincount (Variables|Default|GetTargetGrainCount))
  (bind _scorepergrain (Variables|Default|GetScorePerGrain))
  (bind _qualitypenalty (Variables|Default|GetQualityPenalty))
  (bind (_outscore _outquality) (Class|RiceMath|GradeShari GrainCount _targetgraincount _scorepergrain _qualitypenalty))
  (return _outscore _outquality))
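; BP_PC_Menu is the player controller for the Little Cooks menu.
; On BeginPlay, for the local controller, it starts music through BP_GameInstance_Cooked, shows the mouse cursor, switches to UI-only input and adds a WBP_Menu widget to the viewport.
; The music, cursor and menu setup all depend on the game instance cast succeeding.
; An Escape key binding quits the game.
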(event EventBeginPlay
  (bind _self self)
  (if (Pawn|IsLocalPlayerController)
    (bind _asbp_game_instance_cooked (Utilities|Casting|CastToBP_GameInstance_Cooked (Game|GetGameInstance)))
    (Default|StartMusic _asbp_game_instance_cooked)
    (Variables|Default|SetbShowMouseCursor true)
    (Input|SetInputModeUIOnly _self 0 "DoNotLock" false)
    (bind _returnvalue (UserInterface|CreateWidget "/Game/LittleCooks/UI/WBP_Menu.WBP_Menu_C" _self))
    (UserInterface|Viewport|AddtoViewport _returnvalue 0)))

(event EventTick
  (params (DeltaSeconds :type Float%20%28single-precision%29)))

(event Input|KeyboardEvents|Escape
  (params (Key :type Key%20Structure))
  (:Pressed
    (Game|QuitGame 0 "Quit" false)))

(fn ConstructionScript)
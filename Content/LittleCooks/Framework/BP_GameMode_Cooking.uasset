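; Game mode for the Little Cooks cooking game that runs a timed round and numbers players as they log in.
; BeginPlay sets the order target and countdown on the game state, then starts looping stage and rain timers.
; The stage timer decrements remaining time and flags the round over at zero.
; The rain timer multicasts batched rice rain through the game state's registry until the stage timer stops.
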(event Custom|Tick1s
  (bind _output_get (Variables|/Game/LittleCooks/Framework/BP_GameState_Cooking.BP_GameState_Cooking_C|SetRemainingTime (stale EventBeginPlay _asbp_game_state_cooking) (- (stale EventBeginPlay _output_get) 1.0)))
  (if (<= _output_get 0.0)
    (Utilities|Time|ClearandInvalidateTimerbyHandle (stale EventBeginPlay _output_get_2))
    (Variables|/Game/LittleCooks/Framework/BP_GameState_Cooking.BP_GameState_Cooking_C|SetbRoundOver (stale EventBeginPlay _asbp_game_state_cooking) true)))

(event Custom|RainTick
  (Development|PrintString "rain tick!!!!" false false)
  (if (> (Utilities|Time|GetTimerRemainingTimebyHandle (Variables|Default|GetTimerHandle_Stage)) 0.0)
    (Variables|Default|SetRainBatchIndex (+ (Variables|Default|GetRainBatchIndex) 1))
    (bind _asbp_game_state_cooking (Utilities|Casting|CastToBP_GameState_Cooking (Game|GetGameState)))
    (Default|GetRegistry _asbp_game_state_cooking)
    (Default|MulticastRainRice (Variables|/Game/LittleCooks/Framework/BP_GameState_Cooking.BP_GameState_Cooking_C|GetRegistry _asbp_game_state_cooking) (Variables|Default|GetRainBatchIndex) (Variables|Default|GetRainCount))
    (else
      (Utilities|Time|ClearandInvalidateTimerbyHandle (Variables|Default|GetTimerHandle_Rain)))))

(event EventBeginPlay
  (bind _asbp_game_state_cooking (Utilities|Casting|CastToBP_GameState_Cooking (Game|GetGameState)))
  (if (not (Variables|/Game/LittleCooks/Framework/BP_GameState_Cooking.BP_GameState_Cooking_C|GetbRoundOver _asbp_game_state_cooking))
    (if (<= (Variables|/Game/LittleCooks/Framework/BP_GameState_Cooking.BP_GameState_Cooking_C|GetRemainingTime _asbp_game_state_cooking) 0.0)
      (Variables|/Game/LittleCooks/Framework/BP_GameState_Cooking.BP_GameState_Cooking_C|SetRemainingTime _asbp_game_state_cooking 0.0)
      (Utilities|Time|ClearandInvalidateTimerbyHandle (Variables|Default|GetTimerHandle_Stage))
      (Utilities|Time|ClearandInvalidateTimerbyHandle (Variables|Default|GetTimerHandle_Rain))
      (Variables|/Game/LittleCooks/Framework/BP_GameState_Cooking.BP_GameState_Cooking_C|SetOrderRequired _asbp_game_state_cooking 5)
      (bind _output_get (Variables|/Game/LittleCooks/Framework/BP_GameState_Cooking.BP_GameState_Cooking_C|SetRemainingTime _asbp_game_state_cooking 9e+01))
      (bind _returnvalue (Utilities|Time|SetTimerbyEvent (delegate Custom|Tick1s) 1.0 true))
      (bind _output_get_2 (Variables|Default|SetTimerHandle_Stage _returnvalue))
      (bind _returnvalue_2 (Utilities|Time|SetTimerbyEvent (delegate Custom|RainTick) (Variables|Default|GetRainInterval) true))
      (Variables|Default|SetTimerHandle_Rain _returnvalue_2))))

(event EventTick
  (params (DeltaSeconds :type Float%20%28single-precision%29)))

(event EventPostLogin
  (params (NewPlayer :type Player%20Controller%20Object%20Reference))
  (Development|PrintString "Hello" false false)
  (bind _asbp_player_state_cooking (Utilities|Casting|CastToBP_PlayerState_Cooking (Variables|/Script/Engine.Controller|GetPlayerState NewPlayer)))
  (Variables|/Game/LittleCooks/Framework/BP_PlayerState_Cooking.BP_PlayerState_Cooking_C|SetPlayerNumber _asbp_player_state_cooking (Variables|Default|GetNextPlayerNumber))
  (Variables|Default|SetNextPlayerNumber (+ (Variables|Default|GetNextPlayerNumber) 1)))

(fn ConstructionScript)